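; Central audio controller Blueprint that exposes one function per game sound event for other Blueprints to call.
; BeginPlay either zeroes MasterVolume when MuteAudio is set or plays the 2D music track.
; Jetpack start and end spawn attached sounds with fade-ins, with start returning its audio component.
; Item pickup plays a sound at world origin, while crafting, upgrade station, inventory scroll and special pickup functions are empty stubs.
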(event `self.ReceiveBeginPlay`
  ;[1 1 1] Main code goes here
  (if (`self.MuteAudio`)
    (set `self.MasterVolume` 0.0)
    (else
      (`self.GlobalSoundTrack`))))

(fn `CraftedBigUpgrade`)

(fn `CraftedObject`)

(fn `GlobalSoundTrack`
  (`GameplayStatics.PlaySound2D` "/Game/Audio/Music/GameMusic.GameMusic" 1.0 1.0 0.0 null null))

(fn `InteractWithUpgradeStation`
  ;[1 1 1] Please test this out in the mechanics level first
)

(fn `JetPackEnd`
  (params (NewParam :type "StaticMeshComponent Object Reference"))
  (bind _returnvalue (`GameplayStatics.SpawnSoundAttached` "/Game/Audio/UpgradeModules/JetPack/Jetpack_Switch_Off_Cue.Jetpack_Switch_Off_Cue" NewParam "None" (0.0 0.0 0.0) (struct) "SnapToTarget" false 1.0 1.0 0.0 null null))
  (`AudioComponent.FadeIn` _returnvalue 0.3 1.0 2.0))

(fn `JetPackStart`
  (params (NewParam :type "StaticMeshComponent Object Reference"))
  (returns (SpawnedSound :type "AudioComponent Object Reference"))
  (bind _returnvalue (`GameplayStatics.SpawnSoundAttached` "/Game/Audio/UpgradeModules/JetPack/Jetpack_Flight_Cue.Jetpack_Flight_Cue" NewParam "None" (0.0 0.0 0.0) (struct) "SnapToTarget" false 1.0 1.0 0.0 null null))
  (`AudioComponent.FadeIn` _returnvalue 0.25 1.0 0.0)
  (return _returnvalue))

(fn `PickUpItem`
  (`GameplayStatics.PlaySoundAtLocation` "/Game/Audio/SoundMasterFolder/CraftJam2/Environments/Box_Breaking_01.Box_Breaking_01" (0.0 0.0 0.0) (struct) 1.0 1.0 0.0 null null null)
  (return))

(fn `PickUpSuperAwesomeItem`)

(fn `ScrollThroughInventory`
  ;[1 1 1] Small click sound for when the mouse hovers over buttons
)

(fn `UserConstructionScript`)