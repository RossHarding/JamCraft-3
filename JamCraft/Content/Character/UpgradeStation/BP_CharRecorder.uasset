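; BP_CharRecorder is a scene-capture preview actor for the upgrade station, showing either a character or an object to a render texture.
; At BeginPlay it hides itself and creates a viewport-sized render target for its SceneCaptureComponent2D.
; While switched on, a timeline update yaws TurningSphere from the player's KBTurnValue; switching off hides it and resets rotation.
; Upgrade crafting mode shows the character, while item crafting mode shows the object.
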(event `self.ReceiveBeginPlay`
  (bind (_returnvalue_x _returnvalue_y) (`KismetMathLibrary.BreakVector2D` (`WidgetLayoutLibrary.GetViewportSize` (`GameplayStatics.GetPlayerController` 0))))
  ;[1 1 1] Comment
  (`SceneComponent.SetVisibility` (`self.Root`) false true)
  (bind _asalpho_character_bp (cast `/Game/Character/AlphoCharacter_BP` (`GameplayStatics.GetPlayerCharacter` 0)))
  (set `self.Char_Ref` _asalpho_character_bp)
  (bind _returnvalue (`KismetRenderingLibrary.CreateRenderTarget2D` (`KismetMathLibrary.FTrunc` _returnvalue_x) (`KismetMathLibrary.FTrunc` _returnvalue_y)))
  (bind _output_get (set `SceneCaptureComponent2D.TextureTarget` _returnvalue (`self.SceneCaptureComponent2D`)))
  (set `self.RenderTexture` _output_get))

(event `CharRecorderOn`
  ;[1 1 1] Comment
  (`SceneComponent.SetVisibility` (`self.Root`) true true)
  (set `self.Turn On` true)
  (`Timeline|Timeline_0` :!label _label
    (:`Update`
      (`SceneComponent.K2_AddLocalRotation` (`self.TurningSphere`) (`KismetMathLibrary.MakeRotator` 0.0 0.0 (* (`/Game/Character/AlphoCharacter_BP.KBTurnValue` (`self.Char_Ref`)) (`self.TurnRate`))) false false))))

(event `CharRecorderOff`
  ;[1 1 1] Comment
  (`SceneComponent.SetVisibility` (`self.Root`) false true)
  (set `self.Turn On` false)
  (`|ExecutionSequence`
    (:`then_0`
      (goto _label :!via `Stop`))
    (:`then_1`
      (`SceneComponent.K2_SetRelativeRotation` :`self` (`self.TurningSphere`)))))

(event `EnableItemCraftingStation`
  ;[1 1 1] Comment
  (set `self.UpgradeCrafting` false)
  (`SceneComponent.SetVisibility` (`self.Character`) false false)
  (`SceneComponent.SetVisibility` (`self.Object`) true false))

(event `EnableUpgradeCraftingStation`
  ;[1 1 1] Comment
  (set `self.UpgradeCrafting` true)
  (`SceneComponent.SetVisibility` (`self.Character`) true false)
  (`SceneComponent.SetVisibility` (`self.Object`) false false))

(fn `UserConstructionScript`)