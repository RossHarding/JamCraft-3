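; BP_GroundBend is a short-lived visual effect actor in which a sphere mesh widens horizontally while fading, then destroys itself.
; BeginPlay creates a dynamic M_GroundBend material instance and opens a gate on Tick.
; Each tick grows X and Y scale and lowers Opacity by fixed frame-rate-dependent steps until a size limit is reached.
; A bass-drop sound node exists but is disconnected, so it never plays.
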(event `self.ReceiveTick`
  (params (DeltaSeconds :type "Float (single-precision)"))
  (bind _sphere (`self.Sphere`))
  (bind (_returnvalue_x _returnvalue_y _returnvalue_z) (`KismetMathLibrary.BreakVector` (`SceneComponent.K2_GetComponentScale` _sphere)))
  (`/Engine/EditorBlueprintResources/StandardMacros.Gate` true :!label _label
    (:`Exit`
      (`SceneComponent.SetWorldScale3D` _sphere (`KismetMathLibrary.MakeVector` (+ _returnvalue_x 0.2) (+ _returnvalue_y 0.2) _returnvalue_z))
      (bind _output_get (set `self.Opacity` (- (`self.Opacity`) 0.2)))
      (`MaterialInstanceDynamic.SetScalarParameterValue` (stale `self.ReceiveBeginPlay` _returnvalue) "Opacity" _output_get)
      (if (>= _returnvalue_y 2.0)
        (`self.K2_DestroyActor`)))))

(event `self.ReceiveBeginPlay`
  (bind _returnvalue (`PrimitiveComponent.CreateDynamicMaterialInstance` (`self.Sphere`) 0 "/Game/Materials/M_GroundBend.M_GroundBend"))
  (goto _label :!via `Open`))

(fn `UserConstructionScript`)